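; BP_AmmEnemy is a projectile actor in the space shooter, named as enemy ammunition.
; Each Tick it moves along its forward vector at Speed, without sweeping.
; Overlapping a non-Pawn actor spawns a particle effect and plays a sound, then destroys it after a short delay.
; Pawn overlaps trigger nothing here, and the Blueprint applies no damage itself.
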(event EventBeginPlay)

(event Collision|EventActorBeginOverlap
  (params (OtherActor :type Actor%20Object%20Reference))
  (Utilities|Casting|CastToPawn OtherActor
    (:CastFailed
      (Effects|SpawnEmitteratLocation "/Engine/Tutorial/SubEditors/TutorialAssets/TutorialParticleSystem.TutorialParticleSystem" (Transformation|GetActorLocation))
      (Audio|PlaySound2D "/Engine/EditorSounds/Notifications/CompileStart_Cue.CompileStart_Cue" 1.0 1.0 0.0 0 0)
      (Utilities|FlowControl|Delay 0.2)
      (Actor|DestroyActor))))

(event EventTick
  (params (DeltaSeconds :type Float%20%28single-precision%29))
  (Transformation|SetActorLocation (+ (Transformation|GetActorLocation) (* (Transformation|GetActorForwardVector) (* DeltaSeconds (Variables|Default|GetSpeed)))) false false))

(fn ConstructionScript)